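; Lobby player state holding each player's nickname and ready flag, keeping the lobby HUD in sync.
; Spawn, destruction, nickname replication and the one-way ready event all refresh BP_LobbyHud through the first local player controller.
; Server-to-multicast and server-to-client named RPC events relay ready and chat updates to the HUD and send kicked players to the Title level.
; CopyProperties carries the nickname into BP_PlayerState.
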(event `self.ReceiveBeginPlay`
  ; 플레이어 state가 생성시점에 lobby ui
  (`self.RefreshLobbyUI`)
  ; 플레이어 state가 소멸 시점에 lobby ui 갱신요청 -> refresh ui
  (add `self.OnDestroyed` (delegate `OnDestroyed_Event`)))

(event `OnDestroyed_Event` :!signature `self.OnDestroyed`
  (params (DestroyedActor :type "Actor Object Reference"))
  ; 플레이어 state가 소멸 시점에 lobby ui 갱신요청 -> refresh ui
  (`self.RefreshLobbyUI`))

(event `self.ReceiveCopyProperties`
  (params (NewPlayerState :type "PlayerState Object Reference"))
  (`parent.ReceiveCopyProperties` null)
  (bind _asbp_player_state (cast `/Game/BluePrints/Game/BP_PlayerState` NewPlayerState))
  (set `/Game/BluePrints/Game/BP_PlayerState.NickName` (`self.NickName`) _asbp_player_state))

(event `S2M HandleReadyButton`
  ; Ready 버튼은 한 번만 가능
  (set `self.bIsReady` true)
  (`self.RefreshLobbyUI`))

(event `S2C KickPlayer`
  ; Kicked by server
  (`GameplayStatics.OpenLevelBySoftObjectPtr` "/Game/Maps/Title.Title"))

(event `S2M_ Enter The Text`
  (params (Context :type Text))
  (`self.RefreshUIChatting` Context))

(fn `OnRep_NickName`
  (`self.RefreshLobbyUI`))

(fn `RefreshLobbyUI`
  (bind _returnvalue (`GameplayStatics.GetPlayerController` 0))
  (`/Engine/EditorBlueprintResources/StandardMacros.IsValid` _returnvalue
    (:`Is Valid`
      (bind _asbp_lobby_hud (cast `/Game/BluePrints/Lobby/BP_LobbyHud` (`PlayerController.GetHUD` _returnvalue)))
      (`/Game/BluePrints/Lobby/BP_LobbyHud.RefreshUI` _asbp_lobby_hud))))

(fn `RefreshUIChatting`
  (params (Context :type Text))
  (bind _asbp_lobby_hud (cast `/Game/BluePrints/Lobby/BP_LobbyHud` (`PlayerController.GetHUD` (`GameplayStatics.GetPlayerController` 0))))
  (`/Game/BluePrints/Lobby/BP_LobbyHud.RefreshUI Chatting` _asbp_lobby_hud Context))

(fn `UserConstructionScript`)