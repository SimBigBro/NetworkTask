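; BP_LobbyHud is the lobby HUD that owns the lobby screen's widget.
; On BeginPlay it creates WBP_Lobby, adds it to the viewport and switches the player controller to UI-only input with a visible cursor.
; RefreshUI and RefreshUIChatting events forward to the widget, the latter passing a chat context, with a validity check only on the general refresh.
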(event `self.ReceiveBeginPlay`
  (bind _returnvalue (`GameplayStatics.GetPlayerController` 0))
  (bind _returnvalue_2 (`|CreateWidget` "/Widget/Lobby/WBP_Lobby.WBP_Lobby_C"))
  (bind _output_get (set `self.Lobby UI` _returnvalue_2))
  (`UserWidget.AddToViewport` _output_get 0)
  (`WidgetBlueprintLibrary.SetInputMode_UIOnlyEx` _returnvalue null)
  (set `PlayerController.bShowMouseCursor` true _returnvalue))

(event `RefreshUI`
  (bind _lobby_ui (`self.Lobby UI`))
  (`/Engine/EditorBlueprintResources/StandardMacros.IsValid` _lobby_ui
    (:`Is Valid`
      (`/Widget/Lobby/WBP_Lobby.RefreshUI` _lobby_ui))))

(event `RefreshUI Chatting`
  (params (Context :type Text))
  (`/Widget/Lobby/WBP_Lobby.RefreshUIChatting` (`self.Lobby UI`) Context))

(fn `UserConstructionScript`)