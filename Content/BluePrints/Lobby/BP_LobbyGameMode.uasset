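; Lobby game mode that names joining players, holds match settings and starts the game once everybody is ready.
; PostLogin gives each lobby player state a numbered "User" nickname, and SaveConfig stores the level and player/AI limits.
; TryStartGame checks every player's ready flag, copies both limits to the GameInstance, then after a short delay runs a ServerTravel console command, with seamless travel enabled at BeginPlay.
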(event `self.ReceiveBeginPlay`
  (set `self.bUseSeamlessTravel` true))

(event `TryStartGame`
  ; 모두 준비가 되면 게임 시작
  (if (`self.IsEverybodyReady`)
    (bind _asbp_game_instance (cast `/Game/BluePrints/BP_GameInstance` (`GameplayStatics.GetGameInstance`)))
    (set `/Game/BluePrints/BP_GameInstance.MaxAiCount` (`self.Max Ai Count`) _asbp_game_instance)
    (set `/Game/BluePrints/BP_GameInstance.MaxPlayerCount` (`self.Max Player Count`) _asbp_game_instance)
    (`KismetSystemLibrary.Delay` 3.0)
    (`KismetSystemLibrary.ExecuteConsoleCommand` (`KismetStringLibrary.Concat_StrStr` "ServerTravel" " " (`self.LevelName`)) null)))

(event `self.K2_PostLogin`
  (params (NewPlayer :type "PlayerController Object Reference"))
  ; set nickname-> 자기가 몇번째인지
  (bind _asbp_lobby_player_state (cast `/Game/BluePrints/Lobby/BP_LobbyPlayerState` (`Controller.PlayerState` NewPlayer)))
  (bind _result (`/Engine/EditorBlueprintResources/StandardMacros.IncrementInt` (`self.IndexNickName`))
    (:`  `
      (set `/Game/BluePrints/Lobby/BP_LobbyPlayerState.NickName` (`|FormatText` "User {Index}" _result) _asbp_lobby_player_state))))

(fn `IsEverybodyReady`
  (returns (Ready :type Boolean))
  (for _array_element (`GameStateBase.PlayerArray` (`GameplayStatics.GetGameState`))
    (bind _asbp_lobby_player_state (cast `/Game/BluePrints/Lobby/BP_LobbyPlayerState` _array_element))
    (if (not (`/Game/BluePrints/Lobby/BP_LobbyPlayerState.bIsReady` _asbp_lobby_player_state))
      (return false)))
  ; 다 돈거면 == 모두 레디 상태
  (return true))

(fn `SaveConfig`
  (params (`In Level Name` :type String) (`In Max Player Count` :type Integer) (`In Max Ai Count` :type Integer))
  (`|ExecutionSequence`
    (:`then_0`
      (set `self.LevelName` (`local.In Level Name`)))
    (:`then_1`
      (set `self.Max Player Count` (`local.In Max Player Count`)))
    (:`then_2`
      (set `self.Max Ai Count` (`local.In Max Ai Count`)))))

(fn `UserConstructionScript`)